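; BP_Enemy is an enemy character Blueprint that shows its health on a head widget.
; On BeginPlay it passes itself to the WBP_Enemy_Head instance in its Widget component as that widget's Role.
; When OnHealthChanged fires, it sets the widget's progress to current health divided by max health.
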(event `self.ReceiveBeginPlay`
  (bind _aswbp_enemy_head (cast `/Game/UMG/WBP_Enemy_Head` (`WidgetComponent.GetWidget` (`self.Widget`))))
  (set `/Game/UMG/WBP_Enemy_Head.Role` self _aswbp_enemy_head))

(event `self.OnHealthChanged`
  (params (NewValue :type "Float (single-precision)") (OldValue :type "Float (single-precision)"))
  (bind _aswbp_enemy_head (cast `/Game/UMG/WBP_Enemy_Head` (`WidgetComponent.GetWidget` (`self.Widget`))))
  (`/Game/UMG/WBP_Enemy_Head.SetProgress` _aswbp_enemy_head (/ (`self.GetHealth`) (`self.GetMaxHealth`))))

(fn `UserConstructionScript`)