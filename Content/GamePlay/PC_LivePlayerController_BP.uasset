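; Player controller Blueprint that adds the WBP_Main widget to the viewport at BeginPlay and provides movement and skill-casting functions.
; MoveTo uses SimpleMoveToLocation with a cursor success effect, while Follow steers the pawn toward a point through movement input.
; Helper functions trace the Visibility channel under the cursor or first finger for a location.
; CastSkillByName forwards to the player RoleBase's SkillComponent with unassigned local target values.
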(event `self.ReceiveBeginPlay`
  (bind _returnvalue (`|CreateWidget` "/Game/UMG/WBP_Main.WBP_Main_C" (`GameplayStatics.GetPlayerController` 0)))
  (`UserWidget.AddToViewport` _returnvalue 0))

(fn `CastSkillByName`
  (params (SkillName :type Name))
  (locals (NewLocalVar :type "Actor Object Reference") (NewLocalVar_0 :type "Vector Structure" :default (0.0 0.0 0.0)))
  (bind _asrole_base (cast `RoleBase` (`GameplayStatics.GetPlayerCharacter` 0)))
  (`SkillComponent.CastSkillByName` (`RoleBase.SkillComponent` _asrole_base) SkillName (`local.NewLocalVar`) (`local.NewLocalVar_0`)))

(fn `Follow`
  (params (Location :type "Vector Structure"))
  (bind _returnvalue (`self.K2_GetPawn`))
  (`Pawn.AddMovementInput` _returnvalue (`KismetMathLibrary.GetDirectionUnitVector` (`self.K2_GetActorLocation` _returnvalue) Location) 1.0 false))

(fn `GetLocationUnderCursor`
  (returns (Hit :type Boolean) (Location :type "Vector Structure"))
  (bind (_bblockinghit _binitialoverlap _time _distance _location) (`GameplayStatics.BreakHitResult` (`self.GetHitResultUnderCursorByChannel` "TraceTypeQuery1")))
  (return _bblockinghit _location))

(fn `GetLocationUnderFinger`
  (returns (Hit :type Boolean) (Location :type "Vector Structure"))
  (bind (_bblockinghit _binitialoverlap _time _distance _location) (`GameplayStatics.BreakHitResult` (`self.GetHitResultUnderFingerByChannel` "Touch1" "TraceTypeQuery1" false)))
  (return _bblockinghit _location))

(fn `MoveTo`
  (params (Location :type "Vector Structure"))
  (`AIBlueprintHelperLibrary.SimpleMoveToLocation` self Location)
  (`NiagaraFunctionLibrary.SpawnSystemAtLocation` "/Game/TopDown/Cursor/FX_Cursor_Success.FX_Cursor_Success" Location))

(fn `UserConstructionScript`)