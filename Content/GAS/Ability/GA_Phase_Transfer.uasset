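; Gameplay ability for a "phase transfer" that hides the owning RoleBase character's mesh while the Phase_Transfer effect tag is active.
; On activation it binds a listener to that tag's count, then applies the Phase_Transfer effect container.
; A nonzero count hides the mesh without affecting child components; zero restores visibility and ends the ability, so the tag drives the ability's lifetime.
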(event `self.K2_ActivateAbility`
  (`AbilitySystemBlueprintLibrary.BindEventWrapperToGameplayTagChanged` (`self.GetAbilitySystemComponentFromActorInfo`) (struct :`TagName` "GAS.EffectTag.Phase_Transfer") (delegate `CustomEvent`) true "AnyCountChange")
  (`self.ApplyEffectContainer` (struct :`TagName` "GAS.AbilityEffectContainer.Phase_Transfer")))

(event `CustomEvent`
  (params (Tag :type "GameplayTag Structure (by ref)") (TagCount :type Integer))
  (if (== TagCount 0)
    (bind _asrole_base (cast `RoleBase` (`self.GetOwningActorFromActorInfo`))
      (:`then`
        (`SceneComponent.SetVisibility` (`Character.Mesh` _asrole_base) true false))
      (:`CastFailed`
        _))
    (`self.K2_EndAbility`)
    (else
      (bind _asrole_base_2 (cast `RoleBase` (`self.GetOwningActorFromActorInfo`)))
      (`SceneComponent.SetVisibility` (`Character.Mesh` _asrole_base_2) false false))))

(event `self.K2_OnEndAbility`
  (params (bWasCancelled :type Boolean))
  (`KismetSystemLibrary.PrintString` "Phase_Transfer End"))